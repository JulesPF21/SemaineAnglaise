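; BP_PanningTable is an interactable table where a player pans a placed BP_FishItem over time.
; Interact checks that the fish can be panned, changes its state and locks the player into interacting.
; Tick then advances Progress at a constant Speed, debug-printing it, and on completion releases the player and sets the fish's next state.
; Grabbing or dropping is allowed only at zero or full progress, and resets it.
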(event EventBeginPlay
  (|CallParentFunction) ; This node is disabled and will not be called.\nDrag off pins to build functionality.
)

(event Collision|EventActorBeginOverlap
  (params (OtherActor :type Actor%20Object%20Reference))
  (|CallParentFunction OtherActor) ; This node is disabled and will not be called.\nDrag off pins to build functionality.
)

(event EventTick
  (params (DeltaSeconds :type Float%20%28single-precision%29))
  (|CallParentFunction DeltaSeconds)
  (if (Variables|Default|GetIs%20Interacting)
    (bind _output_get (Variables|Default|Setprogress (Math|Interpolation|FInterptoConstant (Variables|Default|Getprogress) 1.0 DeltaSeconds (Variables|Settings|GetSpeed))))
    (Development|PrintString (Utilities|String|ToString(Float) _output_get) true true "(R=0.000000,G=0.660000,B=1.000000,A=1.000000)" _output_get)
    (if (== (Variables|Default|Getprogress) 1.0)
      (CallFunction|StopInteraction)
      (bind _asbp_fish_item (Utilities|Casting|CastToBP_FishItem (Variables|Default|GetPlacedObject)))
      (Default|SetState _asbp_fish_item "NewEnumerator6"))))

(event EventGrab/Drop
  (params (Player :type BP%20Third%20Person%20Character%20Object%20Reference))
  (if (CallFunction|CanGrabObject)
    (|CallParentFunction Player)
    (Variables|Default|Setprogress 0.0)))

(event EventInteract
  (params (Player :type BP%20Third%20Person%20Character%20Object%20Reference))
  (bind _asbp_fish_item (Utilities|Casting|CastToBP_FishItem (Variables|Default|GetPlacedObject)))
  (if (Default|CanbePanned _asbp_fish_item)
    (Default|SetState _asbp_fish_item "NewEnumerator5")
    (Default|SetIsInteracting Player true self)
    (Variables|Default|SetInteractingPlaver Player)
    (Variables|Default|SetIs%20Interacting true)))

(event EventStopInteraction
  (Variables|Default|SetIs%20Interacting false)
  (Default|SetIsInteracting (Variables|Default|GetInteractingPlaver) false))

(fn ConstructionScript
  (|CallParentFunction))

(fn CanGrabObject
  (return (or (== (Variables|Default|Getprogress) 0.0) (== 1.0 (Variables|Default|Getprogress)))))