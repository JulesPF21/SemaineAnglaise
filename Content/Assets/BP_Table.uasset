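; BP_Table is a table that holds one object placed by the player through the Grab/Drop event.
; When the player holds another object and the table is empty, it attaches that object to ObjectPos, moves it with MoveComponentTo and clears the player's grab reference.
; Otherwise, an empty-handed interaction calls the player's Grab and clears PlacedObject after a short delay.
; Detach clears it directly, while Tick periodically logs its name for debugging.
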(event Custom|Detach
  (Variables|Default|SetPlacedObject 0))

(event EventBeginPlay)

(event Collision|EventActorBeginOverlap
  (params (OtherActor :type Actor%20Object%20Reference)))

(event EventTick
  (params (DeltaSeconds :type Float%20%28single-precision%29))
  (Utilities|FlowControl|Delay 1.0)
  (Utilities|String|LogString (Utilities|GetObjectName (Variables|Default|GetPlacedObject))))

(event EventGrab/Drop
  (params (Player :type BP%20Third%20Person%20Character%20Object%20Reference))
  (bind (_returnvalue _grabledobject) (Default|GetGrabObject Player))
  (if _returnvalue
    (Utilities|IsValid (Variables|Default|GetPlacedObject)
      (:Is%20Not%20Valid
        (if (not (== _grabledobject self))
          (bind _output_get (Variables|Default|SetPlacedObject _grabledobject))
          (Utilities|String|LogString "Objet attaché")
          (Transformation|AttachComponentToComponent _output_get (Variables|Default|GetObjectPos) "None" "KeepWorld" "KeepWorld" "KeepWorld" true)
          (Components|MoveComponentTo (Variables|/Script/Engine.Actor|GetRootComponent (Variables|Default|GetPlacedObject)) "0, 0, 0" "0, 0, 0" false false 0.2 false)
          (Variables|/Game/ThirdPerson/Blueprints/BP_ThirdPersonCharacter.BP_ThirdPersonCharacter_C|SetGrabledObject Player 0))))
    (else
      (Utilities|IsValid (Variables|Default|GetPlacedObject)
        (:Is%20Valid
          (Default|Grab Player _grabledobject))
        (:Is%20Not%20Valid
          _))
      (Utilities|FlowControl|Delay 0.2)
      (Variables|Default|SetPlacedObject 0))))

(fn ConstructionScript)