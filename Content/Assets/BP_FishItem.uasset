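; BP_FishItem is a fish food item that moves through slicing, panning and frying states.
; SetState stores the new state and picks the static mesh for it: the raw mesh setting, sliced fish or fried sliced fish.
; CanBeSliced, CanBePanned and CanBeFried gate each step by combining a per-state lookup with a flag: Slicables for slicing and panning, Fryable for frying.
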(event Custom|SetState
  (params (State :type BPE_FoodState%20Enum :default "NewEnumerator0"))
  (bind _output_get (Variables|Default|SetState State))
  (Components|StaticMesh|SetStaticMesh (Variables|Default|GetItem) (Utilities|Select :Index _output_get :NewEnumerator0 0 :NewEnumerator1 "/Game/Assets/Blender/SlicedFish/Raw/SlicedFishR.SlicedFishR" :NewEnumerator2 "/Game/Assets/Blender/SlicedFish/Raw/SlicedFishR.SlicedFishR" :NewEnumerator3 "/Game/Assets/Blender/SlicedFish/Fried/SlicedFishF.SlicedFishF" :NewEnumerator4 "/Game/Assets/Blender/SlicedFish/Fried/SlicedFishF.SlicedFishF" :NewEnumerator5 "/Game/Assets/Blender/SlicedFish/Raw/SlicedFishR.SlicedFishR" :NewEnumerator6 "/Game/Assets/Blender/SlicedFish/Fried/SlicedFishF.SlicedFishF")))

(event EventBeginPlay)

(event Collision|EventActorBeginOverlap
  (params (OtherActor :type Actor%20Object%20Reference)))

(event EventTick
  (params (DeltaSeconds :type Float%20%28single-precision%29)))

(fn ConstructionScript
  (|CallParentFunction))

(fn CanbeSliced
  (return (and (Variables|Default|GetSlicables) (Utilities|Select :Index (Variables|Default|GetState) :NewEnumerator0 true :NewEnumerator1 true :NewEnumerator2 false :NewEnumerator3 false :NewEnumerator4 false :NewEnumerator5 false :NewEnumerator6 false))))

(fn CanbePanned
  (return (and (Variables|Default|GetSlicables) (Utilities|Select :Index (Variables|Default|GetState) :NewEnumerator0 false :NewEnumerator1 false :NewEnumerator2 true :NewEnumerator3 false :NewEnumerator4 false :NewEnumerator5 true :NewEnumerator6 false))))

(fn CanbeFried
  (return (and (Variables|Default|GetFryable) (Utilities|Select :Index (Variables|Default|GetState) :NewEnumerator0 false :NewEnumerator1 false :NewEnumerator2 false :NewEnumerator3 true :NewEnumerator4 false :NewEnumerator5 false :NewEnumerator6 true))))