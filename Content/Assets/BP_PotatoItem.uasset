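; BP_PotatoItem is a potato food item that tracks its preparation state through slicing, frying and panning.
; SetState stores the new state and swaps the Cube's material, with materials assigned only for Slicing and Scliced.
; CanBeSliced passes for Raw or Slicing, and CanBeFryed for Scliced or Frying, both also requiring Slicables.
; BeginPlay, overlap and Tick are unused stubs, and construction just calls the parent.
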(event Custom|SetState
  (params (State :type BPE_FoodState%20Enum :default "NewEnumerator0"))
  (bind _output_get (Variables|Default|SetState State))
  (Rendering|Material|SetMaterial (Variables|Default|GetCube) 0 (Utilities|Select :Index _output_get :NewEnumerator0 0 :NewEnumerator1 "/Engine/VREditor/UI/ArrowMaterial.ArrowMaterial" :NewEnumerator2 "/Engine/EditorMaterials/Cascade/CASC_RenderNormal_MAT.CASC_RenderNormal_MAT" :NewEnumerator3 0 :NewEnumerator4 0 :NewEnumerator5 0 :NewEnumerator6 0)))

(event EventBeginPlay)

(event Collision|EventActorBeginOverlap
  (params (OtherActor :type Actor%20Object%20Reference)))

(event EventTick
  (params (DeltaSeconds :type Float%20%28single-precision%29)))

(fn ConstructionScript
  (|CallParentFunction))

(fn CanbeSliced
  (return (and (Variables|Default|GetSlicables) (Utilities|Select :Index (Variables|Default|GetState) :NewEnumerator0 true :NewEnumerator1 true :NewEnumerator2 false :NewEnumerator3 false :NewEnumerator4 false :NewEnumerator5 false :NewEnumerator6 false))))

(fn CanbeFryed
  (return (and (Variables|Default|GetSlicables) (Utilities|Select :Index (Variables|Default|GetState) :NewEnumerator0 false :NewEnumerator1 false :NewEnumerator2 true :NewEnumerator3 true :NewEnumerator4 false :NewEnumerator5 false :NewEnumerator6 false))))