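; Fish and chips assembly station where the player places a fish item and a potato item to produce a combined dish.
; Grab/Drop attaches each held ingredient to its own slot and clears the player's hand, or hands over the spawned dish when empty-handed.
; A delayed Tick check destroys both ingredients once present, then spawns and attaches FishNChips at the final position.
; FishReady blocks further placement and is never reset here.
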(event Custom|Detach
  (Variables|Default|SetPlacedObject1 0))

(event EventBeginPlay)

(event Collision|EventActorBeginOverlap
  (params (OtherActor :type Actor%20Object%20Reference)))

(event EventTick
  (params (DeltaSeconds :type Float%20%28single-precision%29))
  (bind _fianl (Variables|Default|GetFianl))
  (Utilities|FlowControl|Delay 0.1)
  (if (and (Utilities|IsValid (Variables|Default|GetPlacedObject1)) (Utilities|IsValid (Variables|Default|GetPlacedObject2)))
    (Variables|Default|SetFishReady true)
    (Actor|DestroyActor (Variables|Default|GetPlacedObject1))
    (Actor|DestroyActor (Variables|Default|GetPlacedObject2))
    (bind _returnvalue (Game|SpawnActorfromClass "/Game/Assets/FishNChips.FishNChips_C" (Transformation|GetRelativeTransform _fianl) "Undefined" "MultiplyWithRoot" 0 "None" 0))
    (bind _output_get (Variables|Default|SetFinalObject _returnvalue))
    (Transformation|AttachComponentToComponent _output_get _fianl "None" "KeepWorld" "KeepWorld" "KeepWorld" true)
    (Components|MoveComponentTo (Variables|/Script/Engine.Actor|GetRootComponent (Variables|Default|GetFinalObject)) "0, 0, 0" "0, 0, 0" false false 0.2 false)))

(event EventGrab/Drop
  (params (Player :type BP%20Third%20Person%20Character%20Object%20Reference))
  (bind (_returnvalue _grabledobject) (Default|GetGrabObject Player))
  (bind _fishready (Variables|Default|GetFishReady))
  (if _returnvalue
    (Utilities|Casting|CastToBP_FishItem _grabledobject
      (:then
        (if (not _fishready)
          (Utilities|IsValid (Variables|Default|GetPlacedObject1)
            (:Is%20Not%20Valid
              (bind _output_get (Variables|Default|SetPlacedObject1 _grabledobject))
              (Transformation|AttachComponentToComponent _output_get (Variables|Default|GetFishPos) "None" "KeepWorld" "KeepWorld" "KeepWorld" true)
              (Components|MoveComponentTo (Variables|/Script/Engine.Actor|GetRootComponent (Variables|Default|GetPlacedObject1)) "0, 0, 0" "0, 0, 0" false false 0.2 false)
              (Variables|/Game/ThirdPerson/Blueprints/BP_ThirdPersonCharacter.BP_ThirdPersonCharacter_C|SetGrabledObject Player 0 :!label _label)))))
      (:CastFailed
        (Utilities|Casting|CastToBP_PotatoItem _grabledobject)
        (if (not _fishready)
          (Utilities|IsValid (Variables|Default|GetPlacedObject2)
            (:Is%20Not%20Valid
              (bind _output_get_2 (Variables|Default|SetPlacedObject2 _grabledobject))
              (Transformation|AttachComponentToComponent _output_get_2 (Variables|Default|GetChipsPose) "None" "KeepWorld" "KeepWorld" "KeepWorld" true)
              (Components|MoveComponentTo (Variables|/Script/Engine.Actor|GetRootComponent (Variables|Default|GetPlacedObject2)) "0, 0, 0" "0, 0, 0" false false 0.2 false)
              (goto _label))))))
    (else
      (Utilities|IsValid (Variables|Default|GetFianl)
        (:Is%20Valid
          (Default|Grab Player (stale EventTick _returnvalue)))
        (:Is%20Not%20Valid
          _))
      (Utilities|FlowControl|Delay 0.2)
      (Variables|Default|SetPlacedObject1 0))))

(fn ConstructionScript)