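; Slicing table station where players cut a placed fish or potato item.
; Interact checks that the item can be sliced, changes its state and marks the player as interacting.
; Tick advances Progress at a constant rate, printing it for debug, then ends the interaction and sets the item's next state at completion.
; Interruption keeps progress, and grab/drop works only at zero or full progress, resetting it.
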(event EventBeginPlay
  (|CallParentFunction) ; This node is disabled and will not be called.\nDrag off pins to build functionality.
)

(event Collision|EventActorBeginOverlap
  (params (OtherActor :type Actor%20Object%20Reference))
  (|CallParentFunction OtherActor) ; This node is disabled and will not be called.\nDrag off pins to build functionality.
)

(event EventTick
  (params (DeltaSeconds :type Float%20%28single-precision%29))
  (bind _placedobject (Variables|Default|GetPlacedObject))
  (|CallParentFunction DeltaSeconds)
  (if (Variables|Default|GetIs%20Interacting)
    (bind _output_get (Variables|Default|Setprogress (Math|Interpolation|FInterptoConstant (Variables|Default|Getprogress) 1.0 DeltaSeconds (Variables|Default|GetSpeed))))
    (Development|PrintString (Utilities|String|ToString(Float) _output_get) true true "(R=0.000000,G=0.660000,B=1.000000,A=1.000000)" _output_get)
    (if (== (Variables|Default|Getprogress) 1.0)
      (CallFunction|StopInteraction)
      (bind _asbp_fish_item (Utilities|Casting|CastToBP_FishItem _placedobject)
        (:then
          (Default|SetState _asbp_fish_item "NewEnumerator2"))
        (:CastFailed
          (bind _asbp_potato_item (Utilities|Casting|CastToBP_PotatoItem _placedobject))
          (Default|SetState _asbp_potato_item "NewEnumerator2"))))))

(event EventGrab/Drop
  (params (Player :type BP%20Third%20Person%20Character%20Object%20Reference))
  (if (CallFunction|CanGrabObject)
    (|CallParentFunction Player)
    (Variables|Default|Setprogress 0.0)))

(event EventInteract
  (params (Player :type BP%20Third%20Person%20Character%20Object%20Reference))
  (bind _placedobject (Variables|Default|GetPlacedObject))
  (bind _asbp_fish_item (Utilities|Casting|CastToBP_FishItem _placedobject)
    (:then
      (if (Default|CanbeSliced _asbp_fish_item)
        (Default|SetState _asbp_fish_item "NewEnumerator1")
        (Default|SetIsInteracting Player true self :!label _label)
        (Variables|Default|SetInteracting%20Player Player)
        (Variables|Default|SetIs%20Interacting true)))
    (:CastFailed
      (bind _asbp_potato_item (Utilities|Casting|CastToBP_PotatoItem _placedobject))
      (if (Default|CanbeSliced _asbp_potato_item)
        (Default|SetState _asbp_potato_item "NewEnumerator1")
        (goto _label)))))

(event EventStopInteraction
  (Variables|Default|SetIs%20Interacting false)
  (Default|SetIsInteracting (Variables|Default|GetInteracting%20Player) false))

(fn ConstructionScript
  (|CallParentFunction))

(fn CanGrabObject
  (return (or (== (Variables|Default|Getprogress) 0.0) (== 1.0 (Variables|Default|Getprogress)))))